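; BP_KillZone is a box trigger that kills the current attempt's penguin in level 1.
; On overlap, it looks up the current attempt number from the level 1 GameState in the PlayerState's PenguinNums map.
; If the overlapping actor matches that entry, it calls KillPlayer on the PlayerState.
; A LastDeadNum guard limits each zone to one kill per attempt, preventing repeat triggers on re-overlap.
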(event `self.Box.OnComponentBeginOverlap`
  (params (OverlappedComponent :type "PrimitiveComponent Object Reference") (OtherActor :type "Actor Object Reference") (OtherComp :type "PrimitiveComponent Object Reference") (OtherBodyIndex :type Integer) (bFromSweep :type Boolean) (SweepResult :type "HitResult Structure (by ref)"))
  (bind _asbp_lvl_1_game_state (cast `/Game/BUT_WHY/Blueprints/Base/BP_lvl1_GameState` (`GameplayStatics.GetGameState`)))
  (bind _asbp_lvl_1_player_state (cast `/Game/BUT_WHY/Blueprints/Base/BP_lvl1_PlayerState` (`GameplayStatics.GetPlayerState` 0)))
  (bind _currentattemptnum (`/Game/BUT_WHY/Blueprints/Base/BP_lvl1_GameState.CurrentAttemptNum` _asbp_lvl_1_game_state))
  (bind (_value _returnvalue) (`BlueprintMapLibrary.Map_Find` (`/Game/BUT_WHY/Blueprints/Base/BP_lvl1_PlayerState.PenguinNums` _asbp_lvl_1_player_state) _currentattemptnum))
  (if _returnvalue
    (if (== OtherActor _value)
      ; Fix for re-overlap
      (if (> _currentattemptnum (`self.LastDeadNum`))
        (set `self.LastDeadNum` _currentattemptnum)
        (`/Game/BUT_WHY/Blueprints/Base/BP_lvl1_PlayerState.Kill Player` _asbp_lvl_1_player_state "NewEnumerator2")))))

(fn `UserConstructionScript`)