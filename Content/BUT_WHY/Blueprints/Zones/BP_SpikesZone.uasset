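; Spike hazard zone that kills the current attempt's penguin when it overlaps the box.
; The construction script scatters instanced spike meshes across a quad between four corner components, with count based on box bounds.
; Spikes mostly follow the Arrow's direction with slight random tilt and size variation, compensating for actor rotation and scale.
; On overlap, it matches the actor against PlayerState's penguin map and calls KillPlayer, using LastDeadNum to prevent repeat kills.
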(event `self.Box.OnComponentBeginOverlap`
  (params (OverlappedComponent :type "PrimitiveComponent Object Reference") (OtherActor :type "Actor Object Reference") (OtherComp :type "PrimitiveComponent Object Reference") (OtherBodyIndex :type Integer) (bFromSweep :type Boolean) (SweepResult :type "HitResult Structure (by ref)"))
  (bind _asbp_lvl_1_game_state (cast `/Game/BUT_WHY/Blueprints/Base/BP_lvl1_GameState` (`GameplayStatics.GetGameState`)))
  (bind _asbp_lvl_1_player_state (cast `/Game/BUT_WHY/Blueprints/Base/BP_lvl1_PlayerState` (`GameplayStatics.GetPlayerState` 0)))
  (bind _currentattemptnum (`/Game/BUT_WHY/Blueprints/Base/BP_lvl1_GameState.CurrentAttemptNum` _asbp_lvl_1_game_state))
  (bind (_value _returnvalue) (`BlueprintMapLibrary.Map_Find` (`/Game/BUT_WHY/Blueprints/Base/BP_lvl1_PlayerState.PenguinNums` _asbp_lvl_1_player_state) _currentattemptnum))
  (if _returnvalue
    (if (== OtherActor _value)
      ; Fix for re-overlap
      (if (> _currentattemptnum (`self.LastDeadNum`))
        (set `self.LastDeadNum` _currentattemptnum)
        (`/Game/BUT_WHY/Blueprints/Base/BP_lvl1_PlayerState.Kill Player` _asbp_lvl_1_player_state "NewEnumerator2")))))

(fn `UserConstructionScript`
  (bind (_returnvalue_location _returnvalue_rotation _returnvalue_scale) (`KismetMathLibrary.BreakTransform` (`KismetMathLibrary.InvertTransform` (`self.GetTransform`))))
  (for _ (range (+ (`KismetMathLibrary.FTrunc` (* (`.SphereRadius` (`KismetSystemLibrary.GetComponentBounds` (`self.Box`))) 0.1)) 1))
    (set `self.RandomU` (`KismetMathLibrary.RandomFloatInRange` 0.0 1.0))
    (set `self.RandomV` (`KismetMathLibrary.RandomFloatInRange` 0.0 1.0))
    (`InstancedStaticMeshComponent.AddInstance` (`self.InstancedStaticMesh`) (`KismetMathLibrary.MakeTransform` (`KismetMathLibrary.VLerp` (`KismetMathLibrary.VLerp` (`SceneComponent.RelativeLocation` (`self.TopLeft`)) (`SceneComponent.RelativeLocation` (`self.TopRight`)) (`self.RandomU`)) (`KismetMathLibrary.VLerp` (`SceneComponent.RelativeLocation` (`self.BottomLeft`)) (`SceneComponent.RelativeLocation` (`self.BottomRight`)) (`self.RandomU`)) (`self.RandomV`)) (`KismetMathLibrary.RLerp` (`KismetMathLibrary.RandomRotator` false) (`KismetMathLibrary.ComposeRotators` (`KismetMathLibrary.Conv_VectorToRotator` (`SceneComponent.GetForwardVector` (`self.Arrow`))) _returnvalue_rotation) 0.97) (* _returnvalue_scale (`KismetMathLibrary.RandomFloatInRange` 0.4 0.6))) false)))