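; Player character with a belly-roll slide, slipping on ice, a timed stun, and interaction input forwarded to an interactable component.
; The slide, available once the game starts, crouches and drives the character forward on a timeline at boosted speed with controller input disabled.
; A downward physical-material trace detects surface changes.
; Moving on ice without sliding or crouching triggers a timeline-driven slip that ends in a stun.
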(event `StopSliding`
  (`|ExecutionSequence`
    (:`then_0`
      (`Timeline|Timeline` :!via `Stop` :!label _label
        (:`Update`
          (`self.AddMovementInput` (`self.GetActorForwardVector`)))
        (:`Finished`
          (set `CharacterMovementComponent.MaxWalkSpeed` (`self.OriginalMaxWalkSpeed`) (`self.CharacterMovement`) :!label _label_2)
          (`|ExecutionSequence`
            (:`then_0`
              (if (not (`self.isStunned`))
                (bind _asbp_lvl_1_controller (cast `/Game/BUT_WHY/Blueprints/Base/BP_lvl1_Controller` (`self.GetController`)))
                (`/Game/BUT_WHY/Blueprints/Base/BP_lvl1_Controller.CustomEnableInput` _asbp_lvl_1_controller)))
            (:`then_1`
              (`|ExecutionSequence`
                (:`then_0`
                  (`|ExecutionSequence`
                    (:`then_0`
                      (set `self.isSliding` false)
                      (`self.OnSlidingStop`))
                    (:`then_1`
                      (`self.PlayAnimMontage` "/Game/BUT_WHY/Blueprints/Characters/Penguin/Meshes/Final/Animations/Montages/AnimMontage_Jump_to_Slide.AnimMontage_Jump_to_Slide" -1.0))))
                (:`then_1`
                  (goto _label_4 :!via `Reset`))))))))
    (:`then_1`
      (goto _label_2))))

(event `Slide`
  (bind _asbp_lvl_1_game_state (cast `/Game/BUT_WHY/Blueprints/Base/BP_lvl1_GameState` (`GameplayStatics.GetGameState`) :!label _label_3))
  (if (`/Game/BUT_WHY/Blueprints/Base/BP_GameState.IsGameStarted` _asbp_lvl_1_game_state)
    (`/Engine/EditorBlueprintResources/StandardMacros.DoOnce` false :!label _label_4
      (:`Completed`
        (`GameplayStatics.PlaySoundAtLocation` "/Game/BUT_WHY/Blueprints/Characters/Penguin/Sounds/Dash/Cue_Dash.Cue_Dash" (`self.K2_GetActorLocation`) (struct) 1.0 1.0 0.0 null null null null)
        (`self.UnCrouch`)
        (`self.OnSlidingStart`)
        (`self.PlayAnimMontage` "/Game/BUT_WHY/Blueprints/Characters/Penguin/Meshes/Final/Animations/Montages/AnimMontage_Jump_to_Slide.AnimMontage_Jump_to_Slide")
        (bind _asbp_lvl_1_controller (cast `/Game/BUT_WHY/Blueprints/Base/BP_lvl1_Controller` (`self.GetController`)))
        (`/Game/BUT_WHY/Blueprints/Base/BP_lvl1_Controller.CustomDisableInput` _asbp_lvl_1_controller)
        (`KismetSystemLibrary.Delay` 0.2)
        (set `self.isSliding` true)
        (set `self.OriginalMaxWalkSpeed` (`CharacterMovementComponent.MaxWalkSpeed` (`self.CharacterMovement`)))
        (set `CharacterMovementComponent.MaxWalkSpeed` (* (`self.OriginalMaxWalkSpeed`) 15.0) (`self.CharacterMovement`))
        (goto _label :!via `PlayFromStart`)))))

(event `EnhancedInput|/Game/BUT_WHY/Blueprints/Inputs/IA_BellyRoll`
  (params (ActionValue :type Boolean) (ElapsedSeconds :type "Float (double-precision)") (TriggeredSeconds :type "Float (double-precision)") (InputAction :type "InputAction Object Reference" :default "/Game/BUT_WHY/Blueprints/Inputs/IA_BellyRoll.IA_BellyRoll"))
  (:`Started`
    (goto _label_3)))

(event `self.ReceiveTick`
  (params (DeltaSeconds :type "Float (single-precision)"))
  (bind _currentsurfacetype (`self.CurrentSurfaceType`))
  (`|ExecutionSequence`
    (:`then_0`
      (bind (_surfacetype _isstandingonsurface) (`self.TraceForSurface`))
      (set `self.OldSurfaceType` _currentsurfacetype)
      (if (not (`|EnumEquality` _surfacetype _currentsurfacetype))
        (bind _output_get (set `self.CurrentSurfaceType` _surfacetype))
        (`self.onMaterialChanged` _output_get _isstandingonsurface (`self.OldSurfaceType`))))))

(event `self.ReceivePossessed`
  (params (NewController :type "Controller Object Reference"))
  (bind _asbp_lvl_1_controller (cast `/Game/BUT_WHY/Blueprints/Base/BP_lvl1_Controller` NewController))
  (add `/Game/BUT_WHY/Blueprints/Base/BP_lvl1_Controller.onMoveStart` _asbp_lvl_1_controller (delegate `OnMoveStart`))
  (add `self.OnSlidingStop` (delegate `Test`)))

(event `OnMoveStart`
  (params (InputVector :type "Vector2D Structure"))
  (bind (_x _y) (`KismetMathLibrary.BreakVector2D` InputVector))
  (bind _returnvalue (`KismetMathLibrary.Normal` (+ (* (`SceneComponent.GetForwardVector` (`self.SpringArm`)) _x) (* _y (`SceneComponent.GetRightVector` (`self.SpringArm`))))))
  (if (not (`self.isStunned`))
    (bind _surfacetype (`self.TraceForSurface`))
    (switch `EPhysicalSurface` _surfacetype
      (:`SurfaceType1`
        (if (not (or (`self.isSliding`) (`NavMovementComponent.IsCrouching` (`self.CharacterMovement`)))) :!label _label_5
          (`/Engine/EditorBlueprintResources/StandardMacros.DoOnce` false :!label _label_6
            (:`Completed`
              (bind _output_get (set `self.isSlipped` true))
              (`KismetSystemLibrary.PrintString` "Hello" _output_get)
              (`|ExecutionSequence`
                (:`then_1`
                  (`Timeline|SlippingTimeline` :!via `PlayFromStart` :!label _label_7
                    (:`Update`
                      (bind _asbp_lvl_1_controller (cast `/Game/BUT_WHY/Blueprints/Base/BP_lvl1_Controller` (`self.GetController`)))
                      (`/Game/BUT_WHY/Blueprints/Base/BP_lvl1_Controller.CustomDisableInput` _asbp_lvl_1_controller)
                      (`self.AddMovementInput` (select `bool` (> (`KismetMathLibrary.VSize` _returnvalue) 0.0) :`false` (`self.GetActorForwardVector`) :`true` _returnvalue))
                      (bind _surfacetype_2 (`self.TraceForSurface`))
                      (switch `EPhysicalSurface` _surfacetype_2
                        (:`SurfaceType_Default`
                          (`|ExecutionSequence`
                            (:`then_0`
                              (goto _label_7 :!via `Stop`))
                            (:`then_1`
                              _)))))
                    (:`Finished`
                      _))
                  (set `self.isSlipped` false :!label _label_8)
                  (`self.Stun`)
                  (bind _asbp_lvl_1_controller_2 (cast `/Game/BUT_WHY/Blueprints/Base/BP_lvl1_Controller` (`self.GetController`))
                    (:`then`
                      (`/Game/BUT_WHY/Blueprints/Base/BP_lvl1_Controller.CustomEnableInput` _asbp_lvl_1_controller_2)
                      (goto _label_6 :!via `Reset`))
                    (:`CastFailed`
                      (goto _label_6 :!via `Reset`))))))))))))

(event `OnMaterialChanged`
  (params (SurfaceType :type "EPhysicalSurface Enum" :default "SurfaceType_Default") (isStandingOnSurface :type Boolean) (SurfaceTypeOld :type "EPhysicalSurface Enum" :default "SurfaceType_Default"))
  (if isStandingOnSurface
    (switch `EPhysicalSurface` SurfaceType
      (:`SurfaceType_Default`
        (if (and (`self.isSliding`) (`|EnumEquality` SurfaceTypeOld "SurfaceType1"))
          (`|ExecutionSequence`
            (:`then_0`
              (`self.StopSliding`)
              (bind _asbp_lvl_1_controller (cast `/Game/BUT_WHY/Blueprints/Base/BP_lvl1_Controller` (`self.GetController`)))
              (`/Game/BUT_WHY/Blueprints/Base/BP_lvl1_Controller.CustomDisableInput` _asbp_lvl_1_controller))
            (:`then_2`
              ; stop timeline
              (`|ExecutionSequence`
                (:`then_0`
                  (goto _label_7 :!via `Stop`))
                (:`then_1`
                  (goto _label_8)))))))
      (:`SurfaceType1`
        (goto _label_5)))))

(event `self.ReceiveBeginPlay`
  (add `self.LandedDelegate` (delegate `Landed`)))

(event `Landed` :!signature `self.LandedDelegate`
  (params (Hit :type "HitResult Structure (by ref)"))
  (if (not (`self.isSliding`))
    (switch `EPhysicalSurface` (`self.CurrentSurfaceType`)
      (:`SurfaceType1`
        ; stop timeline
        (`|ExecutionSequence`
          (:`then_0`
            (goto _label_7 :!via `Stop`))
          (:`then_1`
            (goto _label_8)))))))

(event `Test`
  (if (`self.isSlipped`)
    _))

(event `EnhancedInput|/Game/BUT_WHY/Blueprints/Inputs/IA_Interact`
  (params (ActionValue :type Boolean) (ElapsedSeconds :type "Float (double-precision)") (TriggeredSeconds :type "Float (double-precision)") (InputAction :type "InputAction Object Reference" :default "/Game/BUT_WHY/Blueprints/Inputs/IA_Interact.IA_Interact"))
  (:`Completed`
    (if (`/Game/BUT_WHY/Blueprints/Interactable/AC_Interactable.CanInteract` (`self.AC_Interactable`))
      (`/Game/BUT_WHY/Blueprints/Interactable/I_InteractSource.Interact` (`self.AC_Interactable`)))))

(event `EnhancedInput|/Game/BUT_WHY/Blueprints/Inputs/IA_SpecialInteract`
  (params (ActionValue :type Boolean) (ElapsedSeconds :type "Float (double-precision)") (TriggeredSeconds :type "Float (double-precision)") (InputAction :type "InputAction Object Reference" :default "/Game/BUT_WHY/Blueprints/Inputs/IA_SpecialInteract.IA_SpecialInteract"))
  (:`Started`
    (if (`/Game/BUT_WHY/Blueprints/Interactable/AC_Interactable.CanInteract` (`self.AC_Interactable`))
      (`/Game/BUT_WHY/Blueprints/Interactable/AC_Interactable.SpecialInteract` (`self.AC_Interactable`)))))

(fn `TraceForSurface`
  (returns (SurfaceType :type "EPhysicalSurface Enum") (IsStandingOnSurface :type Boolean))
  (bind (_origin _boxextent) (`KismetSystemLibrary.GetComponentBounds` (`self.CapsuleComponent`)))
  (bind (_outhit _returnvalue) (`KismetSystemLibrary.LineTraceSingle` _origin (- _origin (`KismetMathLibrary.MakeVector` 0.0 0.0 (+ (.z _boxextent) 15.0))) "TraceTypeQuery1"))
  (if _returnvalue
    (bind (_bblockinghit _binitialoverlap _time _distance _location _impactpoint _normal _impactnormal _physmat) (`GameplayStatics.BreakHitResult` _outhit))
    (if (`KismetSystemLibrary.IsValid` _physmat)
      (if true
        (return (`PhysicalMaterial.SurfaceType` _physmat) true))
      (else
        (return "SurfaceType_Default" true)))
    (else
      (return (`self.CurrentSurfaceType`) false))))

(fn `UserConstructionScript`)