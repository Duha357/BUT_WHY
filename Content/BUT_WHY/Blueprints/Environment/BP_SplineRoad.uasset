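; BP_SplineRoad is an environment actor that builds a road along an editable spline.
; Its construction script divides the spline length by a mesh length variable and adds a spline mesh component per segment, forward on X.
; Each segment takes local positions and tangents at its start and end distances, with tangents clamped to the mesh length.
; The event graph holds only disabled stubs, so there is no runtime logic.
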(fn `UserConstructionScript`
  (bind _meshlenght (`self.MeshLenght`))
  (for _index (range (+ (`KismetMathLibrary.FTrunc` (/ (`SplineComponent.GetSplineLength` (`self.Spline`)) (`self.MeshLenght`))) 1))
    (bind _returnvalue (`AddComponent|NODE_AddSplineMeshComponent-1`))
    (`SplineMeshComponent.SetForwardAxis` _returnvalue "X" true)
    (bind _returnvalue_2 (* _index _meshlenght))
    (bind _returnvalue_3 (* (+ _index 1) _meshlenght))
    (`SplineMeshComponent.SetStartAndEnd` _returnvalue (`SplineComponent.GetLocationAtDistanceAlongSpline` (`self.Spline`) _returnvalue_2 "Local") (`KismetMathLibrary.ClampVectorSize` (`SplineComponent.GetTangentAtDistanceAlongSpline` (`self.Spline`) _returnvalue_2 "Local") 0.0 (`self.MeshLenght`)) (`SplineComponent.GetLocationAtDistanceAlongSpline` (`self.Spline`) _returnvalue_3 "Local") (`KismetMathLibrary.ClampVectorSize` (`SplineComponent.GetTangentAtDistanceAlongSpline` (`self.Spline`) _returnvalue_3 "Local") 0.0 (`self.MeshLenght`)) true)))