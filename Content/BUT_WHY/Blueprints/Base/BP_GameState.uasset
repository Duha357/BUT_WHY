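; BP_GameState is a game state Blueprint that runs the countdown timer for a match.
; On BeginPlay it binds its own handler to the GameStart dispatcher and immediately fires it, starting a looping one-second timer.
; Each tick decrements RemainingTime, broadcasts it through the TimerTick dispatcher, and clears the timer once it reaches zero.
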(event `self.ReceiveBeginPlay`
  (add `self.GameStart` (delegate `On Game Start`))
  (`self.GameStart`))

(event `On Game Start`
  (bind _returnvalue (`KismetSystemLibrary.K2_SetTimerDelegate` (delegate `On Timer Tick`) 1.0 true))
  (set `self.RemainingTimer` _returnvalue))

(event `On Timer Tick`
  (bind _output_get (set `self.RemainingTime` (- (`self.RemainingTime`) 1.0)))
  (`self.TimerTick` _output_get)
  (if (<= _output_get 0.0)
    (`KismetSystemLibrary.K2_ClearAndInvalidateTimerHandle` (`self.RemainingTimer`))))

(fn `UserConstructionScript`)