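; Level 1 game state that runs numbered attempts, each with a countdown timer, and handles game pause.
; BeginPlay binds the event handlers and calls game start, which broadcasts the next attempt number.
; Each new attempt resets the remaining time and starts a looping one-second timer that broadcasts ticks and status changes, clearing itself at zero.
; Pause events set the game's paused state, while its own timer tick and status handlers are empty.
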(event `self.ReceiveBeginPlay`
  (`parent.ReceiveBeginPlay`)
  (`|ExecutionSequence`
    (:`then_0`
      (add `self.NewAttempt` (delegate `On New Attempt`)))
    (:`then_1`
      (`self.GameStart`))
    (:`then_2`
      (add `self.GamePause` (delegate `On Game Pause`)))
    (:`then_3`
      (add `self.NewTimerStatus` (delegate `On New Timer Status`)))
    (:`then_4`
      (add `self.TimerTick` (delegate `On Timer Tick`)))))

(event `self.ReceiveTick`
  (params (DeltaSeconds :type "Float (single-precision)"))
  (`parent.ReceiveTick` DeltaSeconds))

(event `On Game Start`
  (`parent.On Game Start`)
  (`self.PlayNextAttempt`))

(event `On New Attempt` :!signature `self.NewAttempt`
  (params (AttemptNum :type Integer))
  (set `self.CurrentAttemptNum` AttemptNum)
  (bind _output_get (set `self.RemainingTime` (`self.DefRemainingTime`)))
  (`self.TimerTick` _output_get)
  (bind _returnvalue (`KismetSystemLibrary.K2_SetTimerDelegate` (delegate `On Local Timer Tick`) 1.0 true))
  (set `self.RemainingTimer` _returnvalue))

(event `On Local Timer Tick`
  (if (`|EnumEquality` (`self.TimerStatus`) "NewEnumerator1")
    (`self.NewTimerStatus` "NewEnumerator0"))
  (bind _output_get (set `self.RemainingTime` (- (`self.RemainingTime`) 1.0)))
  (`self.TimerTick` _output_get)
  (if (<= _output_get 0.0)
    (`self.NewTimerStatus` "NewEnumerator1")
    (`KismetSystemLibrary.K2_ClearAndInvalidateTimerHandle` (`self.RemainingTimer`))))

(event `On Game Pause` :!signature `self.GamePause`
  (params (NewValue :type Boolean))
  (`GameplayStatics.SetGamePaused` NewValue))

(event `On New Timer Status` :!signature `self.NewTimerStatus`
  (params (NewValue :type "/Game/BUT_WHY/Blueprints/Base/Enum/E_TimerStatus Enum" :default "NewEnumerator0")))

(event `On Timer Tick` :!signature `self.TimerTick`
  (params (RemainTime :type "Float (double-precision)")))

(fn `GetNextAttemptNum`
  (returns (NewValue :type Integer))
  (return (+ (`self.CurrentAttemptNum`) 1)))

(fn `PlayNextAttempt`
  (`self.NewAttempt` (`self.GetNextAttemptNum`)))

(fn `UserConstructionScript`)