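; Cutscene manager Blueprint that plays and skips Level Sequence cutscenes by key.
; On BeginPlay it creates a sequence player for every SequenceList entry and stores it under the same key in SequencePlayerList.
; PlayCutscene and SkipCutscene look up the player, call Play or Stop on it if valid, and return it.
; An unknown key only prints an error message.
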(event `self.ReceiveBeginPlay`
  (bind (_keypin _valuepin) (`|MapForEach` (`self.SequenceList`))
    (:`then`
      (bind (_outactor _returnvalue) (`LevelSequencePlayer.CreateLevelSequencePlayer` _valuepin))
      (`BlueprintMapLibrary.Map_Add` (`self.SequencePlayerList`) _keypin _returnvalue))))

(fn `PlayCutscene`
  (params (Key :type Name :default "Intro"))
  (returns (ReturnValue :type "LevelSequencePlayer Object Reference"))
  (bind (_value _returnvalue) (`BlueprintMapLibrary.Map_Find` (`self.SequencePlayerList`) Key))
  (if _returnvalue
    (`/Engine/EditorBlueprintResources/StandardMacros.IsValid` _value
      (:`Is Valid`
        (`MovieSceneSequencePlayer.Play` _value)
        (return _value)))
    (else
      (`KismetSystemLibrary.PrintString` "Cutscene NOT exist!"))))

(fn `SkipCutscene`
  (params (Key :type Name :default "Intro"))
  (returns (ReturnValue :type "LevelSequencePlayer Object Reference"))
  (bind (_value _returnvalue) (`BlueprintMapLibrary.Map_Find` (`self.SequencePlayerList`) Key))
  (if _returnvalue
    (`/Engine/EditorBlueprintResources/StandardMacros.IsValid` _value
      (:`Is Valid`
        (`MovieSceneSequencePlayer.Stop` _value)
        (return _value)))
    (else
      (`KismetSystemLibrary.PrintString` "Cutscene NOT exist!"))))

(fn `UserConstructionScript`)