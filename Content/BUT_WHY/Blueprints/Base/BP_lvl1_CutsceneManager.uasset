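; Level 1 cutscene manager that is set up to signal game start when a cutscene finishes.
; OnFinish casts the game state to BP_lvl1_GameState and calls CallGameStart.
; The logic that plays the "Intro" cutscene and binds OnFinish to its stop event is disconnected and never runs.
; BeginPlay only calls the parent, so nothing in this graph starts the cutscene or triggers OnFinish.
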(event `self.ReceiveBeginPlay`
  (`parent.ReceiveBeginPlay`))

(event `On Finish`
  (bind _asbp_lvl_1_game_state (cast `/Game/BUT_WHY/Blueprints/Base/BP_lvl1_GameState` (`GameplayStatics.GetGameState`)))
  (`/Game/BUT_WHY/Blueprints/Base/BP_GameState.GameStart` _asbp_lvl_1_game_state))

(fn `UserConstructionScript`
  (`parent.UserConstructionScript`))