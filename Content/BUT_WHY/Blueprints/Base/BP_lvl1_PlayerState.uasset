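; Level 1 player state that manages a separate penguin pawn for each attempt, stored in a map by attempt number.
; It listens to level 1 game state timer and attempt events.
; A specific timer status spawns the next attempt's penguin at the player start and steps the life status through two values a second apart.
; Each attempt after the first possesses its mapped penguin and updates life status again.
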(event `self.ReceiveBeginPlay`
  (`parent.ReceiveBeginPlay`)
  (`|ExecutionSequence`
    (:`then_0`
      (bind _asbp_lvl_1_game_state (cast `/Game/BUT_WHY/Blueprints/Base/BP_lvl1_GameState` (`GameplayStatics.GetGameState`)))
      (`|ExecutionSequence`
        (:`then_0`
          (add `/Game/BUT_WHY/Blueprints/Base/BP_lvl1_GameState.NewTimerStatus` _asbp_lvl_1_game_state (delegate `On New Timer Status`)))
        (:`then_1`
          (add `/Game/BUT_WHY/Blueprints/Base/BP_lvl1_GameState.NewAttempt` _asbp_lvl_1_game_state (delegate `On New Attmpt`)))))
    (:`then_1`
      (bind _asbp_penguin (cast `/Game/BUT_WHY/Blueprints/Characters/Penguin/BP_Penguin` (`Controller.K2_GetPawn` (`self.GetPlayerController`))))
      (`BlueprintMapLibrary.Map_Add` (`self.PenguinNums`) 1 _asbp_penguin))))

(event `self.ReceiveTick`
  (params (DeltaSeconds :type "Float (single-precision)"))
  (`parent.ReceiveTick` DeltaSeconds))

(event `self.On Life Status Changed`
  (params (NewValue :type "/Game/BUT_WHY/Blueprints/Base/Enum/E_LifeStatus Enum" :default "NewEnumerator0"))
  (`parent.On Life Status Changed` NewValue))

(event `On New Timer Status`
  (params (NewValue :type "/Game/BUT_WHY/Blueprints/Base/Enum/E_TimerStatus Enum" :default "NewEnumerator0"))
  (if (`|EnumEquality` NewValue "NewEnumerator1")
    (`|ExecutionSequence`
      (:`then_0`
        (bind _asbp_lvl_1_game_state (cast `/Game/BUT_WHY/Blueprints/Base/BP_lvl1_GameState` (`GameplayStatics.GetGameState`)))
        (bind _returnvalue (+ (`/Game/BUT_WHY/Blueprints/Base/BP_lvl1_GameState.CurrentAttemptNum` _asbp_lvl_1_game_state) 1))
        (bind _returnvalue_2 (`|SpawnActorFromClass` "/Game/BUT_WHY/Blueprints/Characters/Penguin/BP_Penguin.BP_Penguin_C" (`self.GetTransform` (`GameModeBase.K2_FindPlayerStart` (`GameplayStatics.GetGameMode`) (`self.GetPlayerController`) "")) "Undefined" "MultiplyWithRoot" null _returnvalue null))
        (`BlueprintMapLibrary.Map_Add` (`self.PenguinNums`) _returnvalue _returnvalue_2))
      (:`then_1`
        (`self.PlayerLifeStatusChanged` "NewEnumerator2")
        (`KismetSystemLibrary.Delay` 1.0)
        (`self.PlayerLifeStatusChanged` "NewEnumerator1")))))

(event `On New Attmpt`
  (params (AttemptNum :type Integer))
  (if (!= AttemptNum 1)
    (`Controller.Possess` (`self.GetPlayerController`) (`BlueprintMapLibrary.Map_Find` (`self.PenguinNums`) AttemptNum))
    (`self.PlayerLifeStatusChanged` "NewEnumerator0")))

(fn `UserConstructionScript`)