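; BP_lvl1_HUD is the level 1 HUD, which puts the base UI widget on screen.
; On BeginPlay it creates WBP_lvl1_Base for the first player controller, stores it as UI and adds it to the viewport.
; DrawSelectionPip draws white, scaled text at a bounds-offset screen position, but nothing here calls it.
; DragSelectResult and PassSelectedUnits are empty stubs for unit selection, the former always returning false.
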(event `self.ReceiveBeginPlay`
  ;[0.15 0.15 0.15 0.502] Setup UI
  (bind _returnvalue (`|CreateWidget` "/Game/BUT_WHY/UI/WBP_lvl1_Base.WBP_lvl1_Base_C" (`GameplayStatics.GetPlayerController` 0)))
  (bind _output_get (set `self.UI` _returnvalue))
  (`UserWidget.AddToViewport` _output_get 0))

(fn `DragSelectResult`
  (params (SelectedActors :type "Array of Actor Object Reference (by ref)"))
  (returns (NewParam :type Boolean))
  (return false))

(fn `DrawSelectionPip`
  (params (Text :type String) (X :type "Float (double-precision)") (Y :type "Float (double-precision)") (`Bounds X` :type "Float (double-precision)") (`Bounds Y` :type "Float (double-precision)"))
  (`self.DrawText` Text (struct :`R` 1.0 :`G` 1.0 :`B` 1.0 :`A` 1.0) (- X `Bounds X`) (+ Y `Bounds Y`) null 1.5))

(fn `PassSelectedUnits`
  (returns (Actors :type "Array of Actor Object Reference"))
  (return))

(fn `UserConstructionScript`)