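; BP_IceDoor is an interactable door that opens once, after being activated and then overlapped.
; OnInteract from any source other than BP_Penguin sets IsActivated and enables overlap events on the trigger box.
; A DoOnce-gated overlap handler plays the opening montage and iron door sound.
; When the montage completes, it disables the blocking box's collision and unbinds the overlap event.
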(event `/Game/BUT_WHY/Blueprints/Interactable/I_InteractReceiver.OnInteract`
  (params (Source :type "Actor Object Reference"))
  (cast `/Game/BUT_WHY/Blueprints/Characters/Penguin/BP_Penguin` Source
    (:`CastFailed`
      (set `self.isActivated` true)
      (set `PrimitiveComponent.bGenerateOverlapEvents` true (`self.BoxOverlap`)))))

(event `self.ReceiveBeginPlay`
  (add `PrimitiveComponent.OnComponentBeginOverlap` (`self.BoxOverlap`) (delegate `OverlapBegin`)))

(event `OverlapBegin`
  (params (OverlappedComponent :type "PrimitiveComponent Object Reference") (OtherActor :type "Actor Object Reference") (OtherComp :type "PrimitiveComponent Object Reference") (OtherBodyIndex :type Integer) (bFromSweep :type Boolean) (SweepResult :type "HitResult Structure (by ref)"))
  (if (`self.isActivated`)
    (`/Engine/EditorBlueprintResources/StandardMacros.DoOnce` false
      (:`Completed`
        (`|PlayMontage` (`self.SK_Door`) "/Game/BUT_WHY/Meshes/Environment/IronDoor/AnimMontage_Open.AnimMontage_Open"
          (:`then`
            (`GameplayStatics.PlaySoundAtLocation` "/Game/BUT_WHY/Blueprints/Interactable/IceDoor/Sounds/Cue_IronDoor.Cue_IronDoor" (`self.K2_GetActorLocation`) (struct) 1.0 1.0 0.0 null null null null))
          (:`OnCompleted`
            (`PrimitiveComponent.SetCollisionEnabled` (`self.BoxCollision`) "NoCollision")
            (clear `PrimitiveComponent.OnComponentBeginOverlap` (`self.BoxOverlap`))))))))

(fn `UserConstructionScript`)