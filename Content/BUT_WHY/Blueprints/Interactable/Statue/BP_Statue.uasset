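; BP_Statue is an interactable statue that makes the penguin character perform a "press F" montage toward it.
; On interact, it disables the penguin's input and uses a timeline to smoothly turn the penguin's yaw to face the statue while the montage plays.
; Input returns when the montage completes or is interrupted, and a DoOnce blocks retriggering until the turn finishes.
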(event `/Game/BUT_WHY/Blueprints/Interactable/I_InteractReceiver.OnInteract`
  (params (Source :type "Actor Object Reference"))
  (bind _asbp_penguin (cast `/Game/BUT_WHY/Blueprints/Characters/Penguin/BP_Penguin` Source))
  (set `self.BP_Penguin` _asbp_penguin)
  (`/Engine/EditorBlueprintResources/StandardMacros.DoOnce` false :!label _label
    (:`Completed`
      (`|ExecutionSequence`
        (:`then_0`
          (`/Game/BUT_WHY/Blueprints/Characters/BP_Character.DisableInputAndInputContext` (`self.BP_Penguin`)))
        (:`then_1`
          (set `self.BeginRotation` (`self.K2_GetActorRotation` (`self.BP_Penguin`)))
          (bind (_direction _newtrack_1) (`Timeline|RotateSlow` :!via `PlayFromStart`)
            (:`Update`
              (bind (_returnvalue_roll _returnvalue_pitch _returnvalue_yaw) (`KismetMathLibrary.BreakRotator` (`KismetMathLibrary.RLerp` (`self.BeginRotation`) (`KismetMathLibrary.FindLookAtRotation` (`self.K2_GetActorLocation` (`self.BP_Penguin`)) (`self.K2_GetActorLocation`)) _newtrack_1)))
              (`self.K2_SetActorRotation` (`self.BP_Penguin`) (`KismetMathLibrary.MakeRotator` 0.0 0.0 _returnvalue_yaw) false))
            (:`Finished`
              (goto _label :!via `Reset`))))
        (:`then_2`
          (`|PlayMontage` (`Character.Mesh` (`self.BP_Penguin`)) "/Game/BUT_WHY/Blueprints/Characters/Penguin/Meshes/Final/Animations/Montages/AnimMontage_PressF.AnimMontage_PressF"
            (:`OnCompleted`
              _)
            (:`OnInterrupted`
              _))
          (`/Game/BUT_WHY/Blueprints/Characters/BP_Character.EnableInputAndInputContext` (`self.BP_Penguin`)))))))

(fn `UserConstructionScript`)