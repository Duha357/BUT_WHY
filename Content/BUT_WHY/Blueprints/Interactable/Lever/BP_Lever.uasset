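; BP_Lever is an interactable lever that activates and triggers a linked Platform.
; A DoOnce limits interaction to a single pull, playing the pull montage and a sound.
; When the montage completes, it sets the Platform active, calls TryToUse and binds to OnPlatformArrived.
; On arrival, it waits briefly, calls TryToUse again, then unbinds, giving one automatic follow-up use.
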(event `/Game/BUT_WHY/Blueprints/Interactable/I_InteractReceiver.OnInteract`
  (params (Source :type "Actor Object Reference"))
  (bind _platform (`self.Platform`))
  (`KismetSystemLibrary.PrintString` (`KismetSystemLibrary.GetDisplayName` Source))
  (`/Engine/EditorBlueprintResources/StandardMacros.DoOnce` false
    (:`Completed`
      (`|PlayMontage` (`self.SkeletalMesh`) "/Game/BUT_WHY/Blueprints/Interactable/Lever/Animations/AnimMontage_Pull.AnimMontage_Pull" 1.0 0.0 "None" false
        (:`then`
          (`GameplayStatics.PlaySoundAtLocation` "/Game/BUT_WHY/Blueprints/Interactable/Lever/Sounds/Cue_lever.Cue_lever" (`self.K2_GetActorLocation`) (struct) 1.0 1.0 0.0 null null null null))
        (:`OnCompleted`
          (set `/Game/BUT_WHY/Blueprints/Interactable/MovingPlatform/BP_MovingPlatform.IsActivated` true _platform)
          (`/Game/BUT_WHY/Blueprints/Interactable/MovingPlatform/BP_MovingPlatform.TryToUse` _platform)
          (add `/Game/BUT_WHY/Blueprints/Interactable/MovingPlatform/BP_MovingPlatform.onPlatformArrived` _platform (delegate `onPlatformArrived_Event`)))))))

(event `onPlatformArrived_Event`
  (bind _platform (`self.Platform`))
  (`KismetSystemLibrary.Delay` 3.5)
  (`/Game/BUT_WHY/Blueprints/Interactable/MovingPlatform/BP_MovingPlatform.TryToUse` _platform)
  (remove `/Game/BUT_WHY/Blueprints/Interactable/MovingPlatform/BP_MovingPlatform.onPlatformArrived` _platform (delegate `onPlatformArrived_Event`)))

(fn `UserConstructionScript`)