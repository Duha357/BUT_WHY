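; BP_MovingPlatform_Final is a usable moving platform that hangs on a rope effect tied to the end of a spline.
; On use, if activated, it flags itself as moving, and each tick while moving it updates the rope beam between the spline's end and its attach point.
; On stop it fires the arrived event, which clears the moving flag, fades out audio and plays an arrival sound.
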(event `self.ReceiveBeginPlay`
  (bind _spline (`/Game/BUT_WHY/Blueprints/Interactable/MovingPlatform/BP_Spline.Spline` (`self.Spline`)))
  (`parent.ReceiveBeginPlay`)
  (`|ExecutionSequence`
    (:`then_0`
      (add `self.onPlatformArrived` (delegate `Arrived`))
      (`NiagaraComponent.SetVariablePosition` (`self.RopeEffect`) "BeamEndPosition" (`SceneComponent.K2_GetComponentLocation` (`self.AttachPoint`)) :!label _label)
      (`NiagaraComponent.SetVariablePosition` (`self.RopeEffect`) "BeamStartPosition" (`SplineComponent.GetLocationAtDistanceAlongSpline` _spline (`SplineComponent.GetSplineLength` _spline) "World")))))

(event `Arrived`
  (set `self.isMoving` false))

(event `self.ReceiveTick`
  (params (DeltaSeconds :type "Float (single-precision)"))
  (`parent.ReceiveTick` DeltaSeconds)
  (if (`self.isMoving`)
    (goto _label)))

(event `self.TryToUse`
  (`parent.TryToUse`)
  (if (`self.IsActivated`)
    (set `self.isMoving` true)))

(event `self.onStop`
  (params (ImpactResult :type "HitResult Structure (by ref)") (Time :type "Float (single-precision)"))
  (`KismetSystemLibrary.PrintString` "this is it")
  (`self.onPlatformArrived`)
  (`AudioComponent.FadeOut` (`self.Audio`) 1.0 0.0 "Linear")
  (`GameplayStatics.PlaySoundAtLocation` "/Game/BUT_WHY/Blueprints/Interactable/MovingPlatform/Sounds/Cue_platform_arrived.Cue_platform_arrived" (`self.K2_GetActorLocation`) (struct) 1.0 1.0 0.0 null null null null))

(fn `UserConstructionScript`
  (`parent.UserConstructionScript`))