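; BP_ThinIce is a thin ice interactable that wears out under a moving penguin, though breaking only prints a debug message.
; On overlap it binds to BP_Penguin's movement and landed delegates.
; Non-crouched movement drains durability per update until it breaks, while landing on its Thin Ice surface triggers a one-time break.
; End overlap unbinds landing but binds movement again instead of unbinding it.
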(event `OnIceBreak`
  (`KismetSystemLibrary.PrintString` "You breaked ice you bozo"))

(event `self.ReceiveBeginPlay`)

(event `self.ReceiveActorBeginOverlap`
  (params (OtherActor :type "Actor Object Reference"))
  (`KismetSystemLibrary.PrintString` "Hello")
  (bind _asbp_penguin (cast `/Game/BUT_WHY/Blueprints/Characters/Penguin/BP_Penguin` OtherActor))
  (bind _output_get (set `self.BP_Penguin_Overlapped` _asbp_penguin))
  (add `Character.OnCharacterMovementUpdated` _output_get (delegate `onMovementUpdated`))
  (add `Character.LandedDelegate` (`self.BP_Penguin_Overlapped`) (delegate `OnLandedDelegate`)))

(event `onMovementUpdated`
  (params (DeltaSeconds :type "Float (single-precision)") (OldLocation :type "Vector Structure") (OldVelocity :type "Vector Structure"))
  (if (> (`KismetMathLibrary.VSize` OldVelocity) 0.0)
    (if (not (`NavMovementComponent.IsCrouching` (`Character.CharacterMovement` (`self.BP_Penguin_Overlapped`))))
      (set `self.IceDurability ` (- (`self.IceDurability `) 0.1))
      (if (<= (`self.IceDurability `) 0.0)
        (`/Engine/EditorBlueprintResources/StandardMacros.DoOnce` false
          (:`Completed`
            (`self.OnIceBreak`)))))))

(event `OnLandedDelegate`
  (params (Hit :type "HitResult Structure (by ref)"))
  (if (== (`.HitActor` (`GameplayStatics.BreakHitResult` Hit)) self)
    (bind _surfacetype (`/Game/BUT_WHY/Blueprints/Characters/BP_Character.TraceForSurface` (`self.BP_Penguin_Overlapped`)))
    (switch `EPhysicalSurface` _surfacetype
      (:`SurfaceType2`
        (`/Engine/EditorBlueprintResources/StandardMacros.DoOnce` false
          (:`Completed`
            (`self.OnIceBreak`)))))))

(event `self.ReceiveActorEndOverlap`
  (params (OtherActor :type "Actor Object Reference"))
  (add `Character.OnCharacterMovementUpdated` (`self.BP_Penguin_Overlapped`) (delegate `onMovementUpdated`))
  (remove `Character.LandedDelegate` (`self.BP_Penguin_Overlapped`) (delegate `OnLandedDelegate`)))

(fn `UserConstructionScript`)