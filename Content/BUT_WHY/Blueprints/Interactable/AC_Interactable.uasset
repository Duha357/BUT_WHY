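; Actor component that gives its owner proximity-based interaction with actors implementing I_InteractReceiver.
; At BeginPlay it adds an overlap sphere to the owner, tracking receivers entering or leaving and broadcasting CanInteractChanged.
; On overlap end, CanInteract is set to whether the list is empty.
; Interact and SpecialInteract fire dispatchers, then call OnInteract on tracked receivers: non-statues for Interact, only BP_Statue for SpecialInteract.
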(event `self.ReceiveBeginPlay`
  (`|ExecutionSequence`
    (:`then_0`
      (bind _returnvalue (`|AddComponentByClass` :`self` (`self.GetOwner`) :`Class` "/Script/Engine.SphereComponent"))
      (bind _output_get (set `self.IntractableSphere` _returnvalue))
      (`SphereComponent.SetSphereRadius` _output_get 100.0 true)
      (`PrimitiveComponent.SetCollisionResponseToAllChannels` _output_get "ECR_Overlap"))
    (:`then_1`
      (add `PrimitiveComponent.OnComponentBeginOverlap` (`self.IntractableSphere`) (delegate `SphereOverlapBegin`)))
    (:`then_2`
      (add `PrimitiveComponent.OnComponentEndOverlap` (`self.IntractableSphere`) (delegate `SphereOverlapEnd`)))
    (:`then_3`
      (add `self.CanInteractChanged` (delegate `On Can Interact Changed`)))))

(event `SphereOverlapBegin`
  (params (OverlappedComponent :type "PrimitiveComponent Object Reference") (OtherActor :type "Actor Object Reference") (OtherComp :type "PrimitiveComponent Object Reference") (OtherBodyIndex :type Integer) (bFromSweep :type Boolean) (SweepResult :type "HitResult Structure (by ref)"))
  (bind _interactable (`self.Interactable`))
  (bind _asi_interact_receiver (cast `/Game/BUT_WHY/Blueprints/Interactable/I_InteractReceiver` OtherActor))
  (`KismetArrayLibrary.Array_Add` _interactable _asi_interact_receiver)
  (`self.CanInteractChanged` true _interactable))

(event `SphereOverlapEnd`
  (params (OverlappedComponent :type "PrimitiveComponent Object Reference") (OtherActor :type "Actor Object Reference") (OtherComp :type "PrimitiveComponent Object Reference") (OtherBodyIndex :type Integer))
  (bind _interactable (`self.Interactable`))
  (bind _asi_interact_receiver (cast `/Game/BUT_WHY/Blueprints/Interactable/I_InteractReceiver` OtherActor))
  (`KismetArrayLibrary.Array_RemoveItem` _interactable _asi_interact_receiver)
  (`self.CanInteractChanged` (`KismetArrayLibrary.Array_IsEmpty` _interactable) _interactable))

(event `On Can Interact Changed` :!signature `self.CanInteractChanged`
  (params (bCanInteract :type Boolean) (IntractableActor :type "Array of /Game/BUT_WHY/Blueprints/Interactable/I_InteractReceiver Interface (by ref)"))
  (bind _output_get (set `self.CanInteract` bCanInteract))
  (if _output_get
    (set `self.Interactable` IntractableActor)))

(event `/Game/BUT_WHY/Blueprints/Interactable/I_InteractSource.Interact`
  (`self.Interacted`)
  (for _array_element (`self.Interactable`)
    (cast `/Game/BUT_WHY/Blueprints/Interactable/Statue/BP_Statue` _array_element
      (:`CastFailed`
        (`/Game/BUT_WHY/Blueprints/Interactable/I_InteractReceiver.OnInteract` _array_element (`self.GetOwner`))))))

(event `/Game/BUT_WHY/Blueprints/Interactable/I_InteractSource.SpecialInteract`
  (`self.SpecialInteracted`)
  (for _array_element (`self.Interactable`)
    (cast `/Game/BUT_WHY/Blueprints/Interactable/Statue/BP_Statue` _array_element)
    (`/Game/BUT_WHY/Blueprints/Interactable/I_InteractReceiver.OnInteract` _array_element (`self.GetOwner`))))